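; Ball actor for a ping-pong game that moves itself across the XY plane and changes course on collision.
; BeginPlay picks a random, unnormalized direction with non-negative X and Y.
; Tick applies a swept offset scaled by Speed and delta time.
; On a blocking hit it sets a new flat direction via GetReflectionVector, with hit normal and current direction fed into each other's inputs.
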(event EventBeginPlay
  (Variables|Default|SetDirection (Math|Vector|MakeVector (Math|Random|RandomFloat) (Math|Random|RandomFloat) 0.0)))

(event Collision|EventActorBeginOverlap
  (params (OtherActor :type Actor%20Object%20Reference)))

(event EventTick
  (params (DeltaSeconds :type Float%20%28single-precision%29))
  (bind _sweephitresult (Transformation|AddActorWorldOffset (Math|Vector|MakeVector (.x (* DeltaSeconds (* (Variables|Default|GetSpeed) (Variables|Default|GetDirection)))) (.y (* DeltaSeconds (* (Variables|Default|GetSpeed) (Variables|Default|GetDirection)))) 0.0) true))
  (if (.bBlockingHit (Collision|BreakHitResult _sweephitresult))
    (Variables|Default|SetDirection (Math|Vector|MakeVector (.x (Math|Vector|GetReflectionVector (.Normal (Collision|BreakHitResult _sweephitresult)) (Variables|Default|GetDirection))) (.y (Math|Vector|GetReflectionVector (.Normal (Collision|BreakHitResult _sweephitresult)) (Variables|Default|GetDirection))) 0.0))))

(fn ConstructionScript)