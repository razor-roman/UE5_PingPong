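; Game state for a ping pong game that holds the start of play until more than one player is present and a countdown finishes.
; Tick latches AllPlayerConnected once Players exceeds one, then decrements Timer through a one-second Delay and sets PlayingGame when it reaches zero.
; The countdown relies on Delay ignoring re-triggers while pending, and this graph never changes the Players count itself.
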(event EventBeginPlay)

(event EventTick
  (params (DeltaSeconds :type Float%20%28single-precision%29))
  (Utilities|FlowControl|Sequence
    (:then_0
      (if (> (Variables|Default|GetPlayers) 1)
        (Variables|Default|SetAllPlayerConnected true)))
    (:then_1
      (if (Variables|Default|GetAllPlayerConnected)
        (if (== (Variables|Default|GetTimer) 0)
          (Variables|Default|SetPlayingGame true)
          (else
            (Utilities|FlowControl|Delay 1.0)
            (Variables|Default|SetTimer (- (Variables|Default|GetTimer) 1))))))))

(fn ConstructionScript)